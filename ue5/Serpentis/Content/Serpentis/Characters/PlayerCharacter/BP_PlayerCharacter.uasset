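; Player character Blueprint that ties camera control and the crosshair HUD to the game's tutorial and draw phases.
; On BeginPlay it binds to the player game mode's state changes, applies a starting pitch and adds the crosshair widget to the viewport.
; State changes lock the camera's Y axis during Tutorial and Waiting for Draw, then release it on Draw.
; The close-tutorial input action calls OnWidgetClosed.
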(event Custom|OnGameStateChanged_Event
  (params (NewState :type E_GameState%20Enum :default "NewEnumerator0"))
  (switch Utilities|FlowControl|Switch|SwitchonE_GameState NewState
    (:NewEnumerator0
      (Class|PlayerCharacter|SetCameraLockY true :!label _label))
    (:NewEnumerator1
      (goto _label))
    (:NewEnumerator2
      (Class|PlayerCharacter|SetCameraLockY false))))

(event Input|EnhancedActionEvents|EnhancedInputActionIA_CloseTutorial
  (params (ActionValue :type Boolean) (ElapsedSeconds :type Float%20%28double-precision%29) (TriggeredSeconds :type Float%20%28double-precision%29) (InputAction :type Input%20Action%20Object%20Reference :default "/Game/Serpentis/Core/Input/IA_CloseTutorial.IA_CloseTutorial"))
  (Default|CallOnWidgetClosed))

(event EventBeginPlay
  (bind _asgm_player_game_mode (Utilities|Casting|CastToGM_PlayerGameMode (Game|GetGameMode)))
  (EventDispatchers|BindEventtoOnGameStateChanged _asgm_player_game_mode (delegate Custom|OnGameStateChanged_Event))
  (Pawn|Input|AddControllerPitchInput (Variables|Default|GetStartingRotation))
  (bind _returnvalue (UserInterface|CreateWidget "/Game/Serpentis/UI/WB_Crosshair.WB_Crosshair_C"))
  (UserInterface|Viewport|AddtoViewport _returnvalue 0))

(fn ConstructionScript)