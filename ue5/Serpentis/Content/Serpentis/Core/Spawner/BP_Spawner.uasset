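; Enemy spawner actor that keeps a BP_Enemy respawning at its own location.
; On BeginPlay it spawns one enemy with a fixed rotation, ignoring collisions, and stores the reference.
; It binds to the death event on that enemy's CharacterAttributeComponent.
; OnDeath_Event sets a timer that calls DoSpawn again after a random delay between MinInterval and MaxInterval.
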(event Custom|OnDeath_Event
  (Utilities|Time|SetTimerbyFunctionName 0 "DoSpawn" (Math|Random|RandomFloatinRange (Variables|Default|GetMinInterval) (Variables|Default|GetMaxInterval))))

(event EventBeginPlay
  (CallFunction|DoSpawn))

(fn ConstructionScript)

(fn DoSpawn
  (bind _returnvalue (Game|SpawnActorfromClass "/Game/Serpentis/Characters/Enemy/BP_Enemy.BP_Enemy_C" (Math|Transform|MakeTransform (Transformation|GetActorLocation) "0.000000,180.000000,0.000000" "1.000000,1.000000,1.000000") "AlwaysSpawn" "MultiplyWithRoot" 0 0))
  (bind _output_get (Variables|Default|SetSpawnedEnemy _returnvalue))
  (EventDispatchers|BindEventtoOnDeathEvent (Variables|/Script/Serpentis.BaseCharacter|GetCharacterAttributeComponent _output_get) (EventDispatchers|CreateEvent :!event Custom|OnDeath_Event)))