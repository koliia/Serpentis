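; Game mode that runs a quick-draw round through Tutorial, WaitingForDraw, Draw and End states, broadcasting each change.
; SetGameState drives pause and the widgets for each phase, with a random timer during the wait for the draw.
; The player character's widget-closed event ends the tutorial, and its death event leads to the win screen after a delay.
; ChangeScore forwards score updates to the score widget.
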(event Custom|OnDeath_Event
  (Utilities|Time|SetTimerbyEvent (delegate Custom|OnEndStateReached) 4.0))

(event Custom|OnEndStateReached
  (CallFunction|SetGameState "NewEnumerator3"))

(event Custom|OnTutorialClosed
  (CallFunction|SetGameState "NewEnumerator1")
  (EventDispatchers|UnbindallEventsfromOnWidgetClosed (Variables|Default|GetCachedPlayerCharacter)))

(event Custom|OnDrawFired
  (CallFunction|SetGameState "NewEnumerator2"))

(event EventBeginPlay
  (bind _asbp_player_character (Utilities|Casting|CastToBP_PlayerCharacter (Game|GetPlayerCharacter 0)))
  (bind _output_get (Variables|Default|SetCachedPlayerCharacter _asbp_player_character))
  (EventDispatchers|BindEventtoOnDeathEvent (Variables|/Script/Serpentis.BaseCharacter|GetCharacterAttributeComponent (Variables|Default|GetCachedPlayerCharacter)) (delegate Custom|OnDeath_Event))
  (EventDispatchers|BindEventtoOnWidgetClosed _output_get (delegate Custom|OnTutorialClosed))
  (Utilities|FlowControl|Delay 0.2)
  (CallFunction|SetGameState "NewEnumerator0"))

(fn ConstructionScript)

(fn SetGameState
  (params (NewState :type E_GameState%20Enum :default "NewEnumerator0"))
  (bind _output_get (Variables|Default|SetCurrentState NewState))
  (Default|CallOnGameStateChanged _output_get)
  (switch Utilities|FlowControl|Switch|SwitchonE_GameState _output_get
    (:NewEnumerator0
      (Game|SetGamePaused true)
      (bind _returnvalue (UserInterface|CreateWidget "/Game/Serpentis/UI/WB_Tutorial.WB_Tutorial_C" (Game|GetPlayerController 0)))
      (bind _output_get_2 (Variables|Default|SetTutorialWidget _returnvalue))
      (UserInterface|Viewport|AddtoViewport _output_get_2 0))
    (:NewEnumerator1
      (Game|SetGamePaused false)
      (Widget|SetVisibility (Variables|Default|GetTutorialWidget) "Hidden")
      (Utilities|Time|SetTimerbyEvent (EventDispatchers|CreateEvent :!event Custom|OnDrawFired) (Math|Random|RandomFloatinRange (Variables|Difficulty|GetMinDrawTime) (Variables|Difficulty|GetMaxDrawTime)))
      (bind _returnvalue_2 (UserInterface|CreateWidget "/Game/Serpentis/UI/WB_Score.WB_Score_C"))
      (bind _output_get_3 (Variables|Default|SetScoreWidget _returnvalue_2))
      (UserInterface|Viewport|AddtoViewport _output_get_3 0)
      (bind _returnvalue_3 (UserInterface|CreateWidget "/Game/Serpentis/UI/WB_WaitDraw.WB_WaitDraw_C"))
      (bind _output_get_4 (Variables|Default|SetWaitDrawWidget _returnvalue_3))
      (UserInterface|Viewport|AddtoViewport _output_get_4 0))
    (:NewEnumerator2
      (bind _returnvalue_4 (UserInterface|CreateWidget "/Game/Serpentis/UI/WB_Draw.WB_Draw_C"))
      (UserInterface|Viewport|AddtoViewport _returnvalue_4 0)
      (Widget|SetVisibility (Variables|Default|GetWaitDrawWidget) "Hidden"))
    (:NewEnumerator3
      (bind _returnvalue_5 (UserInterface|CreateWidget "/Game/Serpentis/UI/WB_WinScreen.WB_WinScreen_C"))
      (UserInterface|Viewport|AddtoViewport _returnvalue_5 0))))

(fn ChangeScore
  (Default|UpdateScore (Variables|Default|GetScoreWidget)))